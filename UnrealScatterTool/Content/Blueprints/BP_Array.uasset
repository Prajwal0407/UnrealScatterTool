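; BP_Array is a construction-script tool that builds 3D grids of static mesh instances from AssetList entries.
; Each entry gets its own HISM, spaced by mesh bounds plus offset, with seeded random location, rotation and uniform or per-axis scale.
; Per-entry overrides then reposition chosen instances relative to instance 0's location and rotation, and listed indices are removed.
; Optional text components label instance IDs for debugging.
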(fn `UserConstructionScript`
  (bind (_currentdata_transform _currentdata_staticmesh _currentdata_count _currentdata_offset _currentdata_instancetransform _currentdata_removedinstance _currentdata_locationseed _currentdata_rotationseed _currentdata_scaleseed _currentdata_minimumrandomtransform _currentdata_maximumrandomtransform _currentdata_minimumrandomscaleuniform _currentdata_maximumrandomscaleuniform) (break `/UnrealScatterTool/Blueprints/F_AssetData` (`self.CurrentData`)))
  (bind _rotationstream (`self.RotationStream`))
  (bind _scalestream (`self.ScaleStream`))
  (bind (_currentdata_transform_2 _currentdata_staticmesh_2 _currentdata_count_2 _currentdata_offset_2) (break `/UnrealScatterTool/Blueprints/F_AssetData` (`self.CurrentData`)))
  (bind _currenthism (`self.CurrentHISM`))
  (bind (_currentdata_transform_3 _currentdata_staticmesh_3 _currentdata_count_3 _currentdata_offset_3 _currentdata_instancetransform_2 _currentdata_removedinstance_2 _currentdata_locationseed_2 _currentdata_rotationseed_2 _currentdata_scaleseed_2 _currentdata_minimumrandomtransform_2 _currentdata_maximumrandomtransform_2) (break `/UnrealScatterTool/Blueprints/F_AssetData` (`self.CurrentData`)))
  (bind _currentdata_transform_4 (break `/UnrealScatterTool/Blueprints/F_AssetData` (`self.CurrentData`)))
  (bind (_currentdata_transform_5 _currentdata_staticmesh_4 _currentdata_count_4 _currentdata_offset_4 _currentdata_instancetransform_3) (break `/UnrealScatterTool/Blueprints/F_AssetData` (`self.CurrentData`)))
  (bind _drawdebuginstanceid_ (`self.DrawDebugInstanceID?`))
  (bind (_currentdata_transform_6 _currentdata_staticmesh_5 _currentdata_count_5 _currentdata_offset_5 _currentdata_instancetransform_4 _currentdata_removedinstance_3) (break `/UnrealScatterTool/Blueprints/F_AssetData` (`self.CurrentData`)))
  (bind _locationstream (`self.LocationStream`))
  (bind (_x _y _z) (break `IntVector` _currentdata_count_2))
  (bind (_returnvalue_min _returnvalue_max) (break `Box` (`StaticMesh.GetBoundingBox` _currentdata_staticmesh_2)))
  (bind _outinstancetransform (`InstancedStaticMeshComponent.GetInstanceTransform` (`self.CurrentHISM`) 0 false))
  (bind (_returnvalue_x _returnvalue_y _returnvalue_z) (`KismetMathLibrary.BreakVector` (- _returnvalue_max _returnvalue_min)))
  (bind _returnvalue (`KismetMathLibrary.MakeRotator` (`KismetMathLibrary.RandomFloatInRangeFromStream` _rotationstream (.roll (.rotation _currentdata_minimumrandomtransform_2)) (.roll (.rotation _currentdata_maximumrandomtransform_2))) (`KismetMathLibrary.RandomFloatInRangeFromStream` _rotationstream (.pitch (.rotation _currentdata_minimumrandomtransform_2)) (.pitch (.rotation _currentdata_maximumrandomtransform_2))) (`KismetMathLibrary.RandomFloatInRangeFromStream` _rotationstream (.yaw (.rotation _currentdata_minimumrandomtransform_2)) (.yaw (.rotation _currentdata_maximumrandomtransform_2)))))
  (bind _values (`BlueprintMapLibrary.Map_Values` (`self.AssetList`)))
  (for _array_element _values
    (bind _output_get (set `self.CurrentData` _array_element))
    (`KismetMathLibrary.SetRandomStreamSeed` (`self.LocationStream`) (`.LocationSeed_49_07FCD02341C13DFF57E3A3A0B38FBFBB` (break `/UnrealScatterTool/Blueprints/F_AssetData` _output_get)))
    (`KismetMathLibrary.SetRandomStreamSeed` (`self.RotationStream`) (`.RotationSeed_50_FAFFC7094E018CEA8DBAC398898E7494` (break `/UnrealScatterTool/Blueprints/F_AssetData` _output_get)))
    (`KismetMathLibrary.SetRandomStreamSeed` (`self.ScaleStream`) (`.ScaleSeed_51_63086825497138FA4F352BB3BE6FC5AC` (break `/UnrealScatterTool/Blueprints/F_AssetData` _output_get)))
    (bind _returnvalue_2 (`AddComponent|NODE_AddHierarchicalInstancedStaticMeshComponent-0` :`RelativeTransform` _currentdata_transform_4))
    (bind _output_get_2 (set `self.CurrentHISM` _returnvalue_2))
    (`StaticMeshComponent.SetStaticMesh` _output_get_2 _currentdata_staticmesh_2)
    (for _index (range _x)
      (for _index_2 (range _y)
        (for _index_3 (range _z)
          (if (`self.UniformScale? (Random)`)
            (bind _returnvalue_3 (+ (`KismetMathLibrary.MakeVector` (* _index (+ _returnvalue_x (.x _currentdata_offset_2))) (* _index_2 (+ _returnvalue_y (.y _currentdata_offset_2))) (* _index_3 (+ (.z _currentdata_offset_2) _returnvalue_z))) (`KismetMathLibrary.MakeVector` (`KismetMathLibrary.RandomFloatInRangeFromStream` _locationstream (.x (.location _currentdata_minimumrandomtransform_2)) (.x (.location _currentdata_maximumrandomtransform_2))) (`KismetMathLibrary.RandomFloatInRangeFromStream` _locationstream (.y (.location _currentdata_minimumrandomtransform_2)) (.y (.location _currentdata_maximumrandomtransform_2))) (`KismetMathLibrary.RandomFloatInRangeFromStream` _locationstream (.z (.location _currentdata_minimumrandomtransform_2)) (.z (.location _currentdata_maximumrandomtransform_2))))))
            (bind _returnvalue_4 (`InstancedStaticMeshComponent.AddInstance` _currenthism (`KismetMathLibrary.MakeTransform` _returnvalue_3 _returnvalue (`KismetMathLibrary.Conv_DoubleToVector` (`KismetMathLibrary.RandomFloatInRangeFromStream` (`self.ScaleStream`) _currentdata_minimumrandomscaleuniform _currentdata_maximumrandomscaleuniform))) false))
            ; DrawDebug
            (if _drawdebuginstanceid_
              (bind _returnvalue_5 (`AddComponent|NODE_AddTextRenderComponent-1` :`RelativeTransform` (`KismetMathLibrary.MakeTransform` (+ (.location (`InstancedStaticMeshComponent.GetInstanceTransform` (`self.CurrentHISM`) _returnvalue_4 false)) (`self.Debug ID Location (Relative to Mesh)`)) (.rotation (`InstancedStaticMeshComponent.GetInstanceTransform` (`self.CurrentHISM`) _returnvalue_4 false)) (.scale (`InstancedStaticMeshComponent.GetInstanceTransform` (`self.CurrentHISM`) _returnvalue_4 false)))))
              (`TextRenderComponent.K2_SetText` _returnvalue_5 (`KismetTextLibrary.Conv_IntToText` _returnvalue_4))
              (`TextRenderComponent.SetWorldSize` (stale _returnvalue_7) (`self.DebugTextSize`) :!label _label)
              (`TextRenderComponent.SetWorldSize` _returnvalue_5 (`self.DebugTextSize`))
              (`TextRenderComponent.SetVerticalAlignment` (stale _returnvalue_7) "EVRTA_TextCenter")
              (`TextRenderComponent.SetVerticalAlignment` _returnvalue_5 "EVRTA_TextCenter")
              (`TextRenderComponent.SetHorizontalAlignment` (stale _returnvalue_7) "EHTA_Center")
              (`TextRenderComponent.SetHorizontalAlignment` _returnvalue_5 "EHTA_Center")
              (`TextRenderComponent.SetTextRenderColor` (stale _returnvalue_7) (`self.DebugTextColor`))
              (`TextRenderComponent.SetTextRenderColor` _returnvalue_5 (`self.DebugTextColor`)))
            (else
              (bind _returnvalue_6 (`InstancedStaticMeshComponent.AddInstance` _currenthism (`KismetMathLibrary.MakeTransform` _returnvalue_3 _returnvalue (`KismetMathLibrary.MakeVector` (`KismetMathLibrary.RandomFloatInRangeFromStream` _scalestream (.x (.scale _currentdata_minimumrandomtransform_2)) (.x (.scale _currentdata_maximumrandomtransform_2))) (`KismetMathLibrary.RandomFloatInRangeFromStream` _scalestream (.y (.scale _currentdata_minimumrandomtransform_2)) (.y (.scale _currentdata_maximumrandomtransform_2))) (`KismetMathLibrary.RandomFloatInRangeFromStream` _scalestream (.z (.scale _currentdata_minimumrandomtransform_2)) (.z (.scale _currentdata_maximumrandomtransform_2))))) false))
              (if _drawdebuginstanceid_
                (bind _returnvalue_7 (`AddComponent|NODE_AddTextRenderComponent-0` :`RelativeTransform` (`KismetMathLibrary.MakeTransform` (+ (.location (`InstancedStaticMeshComponent.GetInstanceTransform` (`self.CurrentHISM`) _returnvalue_6 false)) (`self.Debug ID Location (Relative to Mesh)`)) (.rotation (`InstancedStaticMeshComponent.GetInstanceTransform` (`self.CurrentHISM`) _returnvalue_6 false)) (.scale (`InstancedStaticMeshComponent.GetInstanceTransform` (`self.CurrentHISM`) _returnvalue_6 false)))))
                (`TextRenderComponent.K2_SetText` _returnvalue_7 (`KismetTextLibrary.Conv_IntToText` _returnvalue_6))
                (goto _label)))))))
    ; Instance transform
    (for _array_element_2 _currentdata_instancetransform_3
      (bind (_id _transform) (break `/UnrealScatterTool/Blueprints/F_InstanceData` _array_element_2))
      (`InstancedStaticMeshComponent.UpdateInstanceTransform` (`self.CurrentHISM`) _id (`KismetMathLibrary.MakeTransform` (+ (.location _transform) (.location _outinstancetransform)) (`KismetMathLibrary.MakeRotator` (+ (.roll (.rotation _transform)) (.roll (.rotation _outinstancetransform))) (+ (.pitch (.rotation _transform)) (.pitch (.rotation _outinstancetransform))) (+ (.yaw (.rotation _transform)) (.yaw (.rotation _outinstancetransform)))) (.scale _transform)) false false false))
    ; Remove Instances
    (for _array_element_3 _currentdata_removedinstance_3
      (`InstancedStaticMeshComponent.RemoveInstance` (`self.CurrentHISM`) _array_element_3))))